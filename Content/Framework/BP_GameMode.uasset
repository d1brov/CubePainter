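; Game mode for a target-painting level that tracks how many targets the player has painted and restarts when all are done.
; On BeginPlay it creates the HUD widget and counts every BP_Target in the level as the goal.
; Increment and decrement functions update the painted count and refresh the widget.
; Each increment runs a win check, which reopens the Stage level once the count reaches the total.
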(event Custom|TargetPainted
  (bind _iswon (CallFunction|IsWon))
  (if _iswon
    (CallFunction|RestartLevel)))

(event EventBeginPlay
  ;[1 1 1] Init UI widget
  (bind _returnvalue (UserInterface|CreateWidget "/Game/UI/BP_Widget.BP_Widget_C" (Game|GetPlayerController 0)))
  (bind _output_get (Variables|Default|SetUiRef _returnvalue))
  (UserInterface|Viewport|AddtoViewport _output_get 0)
  ;[1 1 1] Calculate targets on level
  (bind _outactors (Actor|GetAllActorsOfClass "/Game/GameElements/BP_Target.BP_Target_C"))
  (Variables|Default|SetTargetsAmount (Utilities|Array|Length _outactors))
  (Default|UpdateTargetsAmount (Variables|Default|GetUiRef))
  (Default|UpdatePlayerPaintedTargets (Variables|Default|GetUiRef)))

(fn ConstructionScript)

(fn IncrementPaintedTargets
  (Math|Integer|IncrementInt (Variables|Default|GetPlayerPaintedTargets)
    (:%20%20
      (Default|UpdatePlayerPaintedTargets (Variables|Default|GetUiRef))
      (CallFunction|TargetPainted))))

(fn RestartLevel
  (Game|OpenLevel(byObjectReference) "/Game/Levels/Stage.Stage"))

(fn DecrementPaintedTargets
  (Math|Integer|DecrementInt (Variables|Default|GetPlayerPaintedTargets)
    (:%20%20
      (Default|UpdatePlayerPaintedTargets (Variables|Default|GetUiRef)))))

(fn IsWon
  (return (>= (Variables|Default|GetPlayerPaintedTargets) (Variables|Default|GetTargetsAmount))))