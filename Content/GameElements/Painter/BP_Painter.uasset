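; BP_Painter is a cone game element that holds a paint color and takes on the player's painter color when the player hits it.
; On a hit with a different color, it stores the new color, updates the cone's dynamic material and plays a sound.
; The construction script applies the initial color to the material.
; GetPainterColor exposes the current color, and IsActivePainter always returns true.
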(event OnComponentHit(Cone)
  (params (HitComponent :type Primitive%20Component%20Object%20Reference) (OtherActor :type Actor%20Object%20Reference) (OtherComp :type Primitive%20Component%20Object%20Reference) (NormalImpulse :type Vector :default "0, 0, 0") (Hit :type Hit%20Result%20Structure%20%28by%20ref%29))
  (bind _cone (Variables|Default|GetCone))
  ;[1 1 1] Change painting color if hit by other painter
  (bind _asbp_player (Utilities|Casting|CastToBP_Player OtherActor))
  (bind _paintercolor (Default|GetPainterColor _asbp_player))
  (if (not (== _paintercolor (Variables|Default|GetColor)))
    (bind _output_get (Variables|Default|SetColor _paintercolor))
    (Rendering|Material|CreateDynamicMaterialInstance _cone 0 0 "None" :!class /Script/Engine.PrimitiveComponent)
    (Rendering|Material|SetVectorParameterValueonMaterials _cone "Color" (Math|Conversions|ToVector(LinearColor) _output_get))
    (Audio|PlaySound2D "/Engine/VREditor/Sounds/VR_open_Cue.VR_open_Cue" 1.0 1.0 0.0 0 0)))

(fn ConstructionScript
  (bind _cone (Variables|Default|GetCone))
  (Rendering|Material|CreateDynamicMaterialInstance _cone 0 0 "None" :!class /Script/Engine.PrimitiveComponent)
  (Rendering|Material|SetVectorParameterValueonMaterials _cone "Color" (Math|Conversions|ToVector(LinearColor) (Variables|Default|GetColor))))

(fn GetPainterColor
  (return (Variables|Default|GetColor)))

(fn IsActivePainter
  (return true))