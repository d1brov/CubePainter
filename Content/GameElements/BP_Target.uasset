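; BP_Target is a physics cube that active BI_Painter actors repaint by hitting it, with a dynamic material showing its color.
; On a color change, it compares against the player pawn's color, updates BP_GameMode's painted-target count and plays gain or loss sounds.
; A looping timer with a randomized interval kicks near-stationary cubes with random upward and angular impulses, with a sound.
; It reports itself as a non-active painter and exposes its color.
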(event OnComponentHit(Cube)
  (params (HitComponent :type Primitive%20Component%20Object%20Reference) (OtherActor :type Actor%20Object%20Reference) (OtherComp :type Primitive%20Component%20Object%20Reference) (NormalImpulse :type Vector :default "0, 0, 0") (Hit :type Hit%20Result%20Structure%20%28by%20ref%29))
  ;[1 1 1] Painting logic
  (|Hitbypainter OtherActor)
  (bind _paintercolor (Class|BIPainter|GetPainterColor(Message) OtherActor))
  (|Painterhasdifferentcolor _paintercolor (Variables|Default|GetColor))
  (bind _asbp_game_mode (Utilities|Casting|CastToBP_GameMode (Game|GetGameMode)))
  (bind _paintercolor_2 (Class|BIPainter|GetPainterColor(Message) (Game|Player|GetPlayerPawn 0)))
  (|Painterhasplayercolor _paintercolor_2 _paintercolor
    (:then
      (Default|IncrementPaintedTargets _asbp_game_mode)
      (Audio|PlaySound2D "/Engine/VREditor/Sounds/VR_click1.VR_click1" 1.0 1.0 0.0 0 0))
    (:else
      (|Iftargethadplayercolor _paintercolor_2
        (:then
          (Default|DecrementPaintedTargets _asbp_game_mode)
          (Audio|PlaySound2D "/Engine/VREditor/Sounds/VR_negative.VR_negative" 1.0 1.0 0.0 0 0))
        (:false
          _))))
  (Variables|Default|SetColor _paintercolor)
  (|Paintmesh _paintercolor))

(event Custom|MoveTarget
  (bind _returnvalue (Math|Random|RandomUnitVector))
  ;[1 1 1] Random movement
  ;;[1 1 1] Velocity threshold check
  (if (< (Math|Vector|VectorLength (Transformation|GetVelocity)) 1.0)
    ;;[1 1 1] Add random side & vertical impulse
    (Physics|AddImpulse (Variables|Actor|GetCube) (* (Math|Random|RandomIntegerinRange 0 1500) (Math|Vector|MakeVector (.x _returnvalue) (.y _returnvalue) (Math|Float|Absolute(Float) (.z _returnvalue)))) "None" true)
    ;;[1 1 1] Add little angular impulse
    (Class|PrimitiveComponent|AddAngularImpulseinRadians (Variables|Actor|GetCube) (* (Math|Random|RandomIntegerinRange 0 25) (Math|Random|RandomUnitVector)) "None" true)
    ;;[1 1 1] Play sound on impulse
    (Audio|PlaySoundatLocation "/Engine/VREditor/Sounds/UI/Floating_UI_Close.Floating_UI_Close" (Transformation|GetWorldLocation (Variables|Actor|GetCube)) "0, 0, 0" 0.5 1.0 0.0 0 0 0 0)))

(event EventBeginPlay
  ;[1 1 1] Random movement
  (Utilities|Time|SetTimerbyEvent (delegate Custom|MoveTarget) (Math|Random|RandomFloatinRange 2.0 5.0) true))

(fn ConstructionScript
  (bind _cube (Variables|Actor|GetCube))
  (Rendering|Material|CreateDynamicMaterialInstance _cube 0 0 "None" :!class /Script/Engine.PrimitiveComponent)
  (Rendering|Material|SetVectorParameterValueonMaterials _cube "Color" (Math|Conversions|ToVector(LinearColor) (Variables|Default|GetColor))))

(fn IsActivePainter
  (return false))

(fn GetColor
  (return (Variables|Default|GetColor)))